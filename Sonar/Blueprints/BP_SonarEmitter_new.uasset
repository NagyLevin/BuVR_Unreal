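; Sonar emitter actor that simulates a noisy scanning sonar, mirroring its settings and pose to MPC_Sonar.
; A looping DoPing timer nudges the cone along X and line-traces a ray fan, spawning Niagara echoes.
; Floor hits and misses step through widening box traces or random noise points.
; After movement beyond a threshold, a marker appears and echoes are drawn from the locked origin, which S_LockNewPos updates.
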(event Custom|Debug
  ;[0.15 0.15 0.15 0.5] Debug Zone
)

(event Custom|DoPing
  (bind _returnvalue (Math|Vector|MakeVector 0.0 0.0 1.0))
  (bind _cone_sonar (Variables|Components|GetCone_Sonar))
  (bind _cone_sonar_2 (Variables|Components|GetCone_Sonar))
  (bind _cone_sonar_3 (Variables|Components|GetCone_Sonar))
  (bind _returnvalue_2 (Transformation|GetWorldLocation _cone_sonar))
  (bind _returnvalue_3 (Transformation|GetWorldRotation _cone_sonar_3))
  ;[0.15 0.15 0.15 0.5] Szakdoga
  (Variables|Default|SetE_CurrentEmitterLocation (Transformation|GetWorldLocation (Variables|Components|GetCone_Sonar)))
  (if (Variables|Default|GetE_bLockedLocationInitialized)
    (if (Variables|Default|GetE_FreezeOnLargeTranslation)
      (bind _returnvalue_4 (Rendering|Material|GetScalarParameterValue "/Game/Sonar/MaterialParameterCollection/MPC_Sonar.MPC_Sonar" "S_LockNewPos" :!class /Script/Engine.KismetMaterialLibrary))
      (if (== _returnvalue_4 1.0)
        (Variables|Default|SetE_LockedEmitterLocation (Variables|Default|GetE_CurrentEmitterLocation))
        (Transformation|SetWorldLocation (Variables|Default|GetSonar%20marker) (Variables|Default|GetE_CurrentEmitterLocation) false false)
        (Rendering|Material|SetScalarParameterValue "/Game/Sonar/MaterialParameterCollection/MPC_Sonar.MPC_Sonar" "S_LockNewPos" 1.0 :!class /Script/Engine.KismetMaterialLibrary))
      (else
        (Variables|Default|SetE_TranslationDistance (Math|Vector|Distance(Vector) (Variables|Default|GetE_LockedEmitterLocation) (Variables|Default|GetE_CurrentEmitterLocation)))
        (if (<= (Variables|Default|GetE_TranslationDistance) (Variables|Default|GetE_TranslationThreshold))
          _
          (else
            (Rendering|SetVisibility (Variables|Default|GetSonar%20marker) true false)
            (Variables|Default|SetE_FreezeOnLargeTranslation true)))))
    (else
      (Variables|Default|SetE_LockedEmitterLocation (Variables|Default|GetE_CurrentEmitterLocation))
      (Variables|Default|SetE_bLockedLocationInitialized true)))
  (Transformation|SetWorldLocation (Variables|Components|GetCone_Sonar) (+ (Transformation|GetWorldLocation (Variables|Components|GetCone_Sonar)) "1.000000,0.000000,0.000000") false false)
  (bind _returnvalue_5 (Rendering|Material|GetScalarParameterValue "/Game/Sonar/MaterialParameterCollection/MPC_Sonar.MPC_Sonar" "S_Fov" :!class /Script/Engine.KismetMaterialLibrary))
  (Variables|Default|SetS_FOVAngle (/ _returnvalue_5 2.0))
  (for _index (range 0 (- (Variables|Default|GetS_Numrays) -1))
    (Variables|Default|SetS_RayHitLoc _returnvalue_2)
    (Variables|Default|SetE_DisplayPoint _returnvalue_2)
    (Variables|Default|SetE_DirectionVector (Math|Vector|RotateVectorAroundAxis (Math|Vector|GetForwardVector _cone_sonar_2) (Math|Float|MapRangeClamped (Math|Conversions|ToFloat(Integer) _index) 0.0 (Math|Conversions|ToFloat(Integer) (- (Variables|Default|GetS_Numrays) -1)) (* (* (Variables|Default|GetS_FOVAngle) 0.3) -1.0) (* (Variables|Default|GetS_FOVAngle) 0.3)) (Math|Vector|GetRightVector _cone_sonar_2)))
    (bind (_outhit _returnvalue_6) (Collision|LineTraceByChannel (Variables|Default|GetE_CurrentEmitterLocation) (+ (* (Variables|Default|GetE_DirectionVector) (Variables|Default|GetS_MaxRange)) (Variables|Default|GetE_CurrentEmitterLocation)) "TraceTypeQuery1" false 0 "None"))
    (if _returnvalue_6
      (if (Actor|ActorHasTag (.HitActor (Collision|BreakHitResult _outhit)) "Floor")
        (bind _index_2 (Utilities|FlowControl|ForLoopwithBreak 1 (Variables|Default|GetS_steps) :!label _label)
          (:LoopBody
            (Rendering|Material|GetScalarParameterValue "/Game/Sonar/MaterialParameterCollection/MPC_Sonar.MPC_Sonar" "S_NoiseHitbox" :!class /Script/Engine.KismetMaterialLibrary)
            ;[0.15 0.15 0.15 0.5] Random noise
            (bind _returnvalue_7 (Rendering|Material|GetScalarParameterValue "/Game/Sonar/MaterialParameterCollection/MPC_Sonar.MPC_Sonar" "S_NoiseRange" :!class /Script/Engine.KismetMaterialLibrary))
            (if (< (Math|Random|RandomFloatinRange 0.001 1.0) _returnvalue_7)
              (if true
                (Variables|Default|SetS_RayHitLoc (+ (Variables|Default|GetE_LockedEmitterLocation) (* (Variables|Default|GetE_DirectionVector) (* (Math|Random|RandomFloatinRange 0.0 1.0) (Variables|Default|GetS_MaxRange))))))
              (else
                (if (> (Math|Float|Absolute(Float) (Math|Vector|DotProduct (Math|Vector|GetRightVector _returnvalue_3) _returnvalue)) (Math|Float|Absolute(Float) (Math|Vector|DotProduct (Math|Vector|GetUpVector _returnvalue_3) _returnvalue)))
                  (Variables|Default|SetE_WidehitboxZ (* (* (Math|Conversions|ToFloat(Integer) _index_2) 2e+02) 0.1))
                  (else
                    (Variables|Default|SetE_WidehitboxY (* (* (Math|Conversions|ToFloat(Integer) _index_2) 2e+02) 0.1))))
                (bind (_outhit_2 _returnvalue_8) (Collision|BoxTraceByChannel (Variables|Default|GetE_CurrentEmitterLocation) (+ (* (Variables|Default|GetE_DirectionVector) (* (Math|Conversions|ToFloat(Integer) _index_2) 2e+02)) (Variables|Default|GetE_CurrentEmitterLocation)) (Math|Vector|MakeVector 1.0 (Variables|Default|GetE_WidehitboxY) (Variables|Default|GetE_WidehitboxZ)) (Math|Rotator|MakeRotfromX (Variables|Default|GetE_DirectionVector)) "TraceTypeQuery1" false 0 "ForOneFrame"))
                (if _returnvalue_8
                  (Variables|Default|SetS_RayHitLoc (.Location (Collision|BreakHitResult _outhit_2)))
                  (Variables|Default|SetE_DisplayPoint (.Location (Collision|BreakHitResult _outhit_2)))
                  (Development|PrintString "Got a hit with:")
                  (Development|PrintString (Utilities|String|ToString(Float) (* (Math|Conversions|ToFloat(Integer) _index_2) 2e+02)))
                  (goto _label Break)))))
          (:Completed
            (if (Variables|Default|GetE_FreezeOnLargeTranslation)
              ;[0.15 0.15 0.15 0.5] Szakdoga Hit location offset
              (Variables|Default|SetE_HitDistance (Math|Vector|Distance(Vector) (Variables|Default|GetE_CurrentEmitterLocation) (Variables|Default|GetS_RayHitLoc)) :!label _label_2)
              (Variables|Default|SetE_DisplayPoint (+ (Variables|Default|GetE_LockedEmitterLocation) (* (Variables|Default|GetE_DirectionVector) (Variables|Default|GetE_HitDistance)))))
            (Rendering|Debug|DrawDebugLine "0, 0, 0" "0, 0, 0" "(R=0.000000,G=1.000000,B=0.000000,A=1.000000)" 1.0 1.0 :!label _label_3)
            (Rendering|Debug|DrawDebugLine "0, 0, 0" "0, 0, 0" "(R=1.000000,G=0.000000,B=0.000000,A=1.000000)" 1.0 1.0)
            (Niagara|SpawnSystematLocation "/Game/Sonar/NS_Sonar_Raycast.NS_Sonar_Raycast" (Variables|Default|GetE_DisplayPoint))))
        (else
          (Variables|Default|SetS_RayHitLoc (.Location (Collision|BreakHitResult _outhit)))
          (Variables|Default|SetE_DisplayPoint (.Location (Collision|BreakHitResult _outhit)))
          (if (Variables|Default|GetE_FreezeOnLargeTranslation)
            (goto _label_2)
            (else
              (goto _label_3)))))
      (else
        (goto _label)))))

(event EventBeginPlay
  (bind _returnvalue (Rendering|Material|GetScalarParameterValue "/Game/Sonar/MaterialParameterCollection/MPC_Sonar.MPC_Sonar" "Light" :!class /Script/Engine.KismetMaterialLibrary))
  (if (== _returnvalue 0.0)
    (Variables|Default|SetLights false)
    (else
      (Variables|Default|SetLights true)))
  (bind _returnvalue_2 (Rendering|Material|GetScalarParameterValue "/Game/Sonar/MaterialParameterCollection/MPC_Sonar.MPC_Sonar" "HalfAngleDeg" :!class /Script/Engine.KismetMaterialLibrary))
  (Variables|Default|SetHalfAngleDeg _returnvalue_2)
  (bind _returnvalue_3 (Rendering|Material|GetScalarParameterValue "/Game/Sonar/MaterialParameterCollection/MPC_Sonar.MPC_Sonar" "IMU_DriftRate" :!class /Script/Engine.KismetMaterialLibrary))
  (Variables|Default|SetIMU_DriftRate _returnvalue_3)
  (bind _returnvalue_4 (Rendering|Material|GetScalarParameterValue "/Game/Sonar/MaterialParameterCollection/MPC_Sonar.MPC_Sonar" "Mode" :!class /Script/Engine.KismetMaterialLibrary))
  (Variables|Default|SetMode _returnvalue_4)
  (bind _returnvalue_5 (Rendering|Material|GetScalarParameterValue "/Game/Sonar/MaterialParameterCollection/MPC_Sonar.MPC_Sonar" "NoiseAmp" :!class /Script/Engine.KismetMaterialLibrary))
  (Variables|Default|SetNoiseAmp _returnvalue_5)
  (bind _returnvalue_6 (Rendering|Material|GetScalarParameterValue "/Game/Sonar/MaterialParameterCollection/MPC_Sonar.MPC_Sonar" "PingHz" :!class /Script/Engine.KismetMaterialLibrary))
  (Variables|Default|SetPingHz _returnvalue_6)
  (bind _returnvalue_7 (Rendering|Material|GetScalarParameterValue "/Game/Sonar/MaterialParameterCollection/MPC_Sonar.MPC_Sonar" "Range" :!class /Script/Engine.KismetMaterialLibrary))
  (Variables|Default|SetRange _returnvalue_7)
  (Utilities|Time|SetTimerbyFunctionName 0 "DoPing" 0.05 true)
  (Utilities|Time|SetTimerbyFunctionName 0 "Debug" 0.5 true)
  (Transformation|SetWorldRotation (Variables|Components|GetCone_Sonar) (Transformation|GetActorRotation) false false)
  (Variables|Default|SetE_LockedEmitterLocation (Transformation|GetWorldLocation (Variables|Components|GetCone_Sonar)))
  (Variables|Default|SetE_bLockedLocationInitialized true)
  ;[0.15 0.15 0.15 0.5] Make reference cone invis
  (Rendering|SetVisibility (Variables|Default|GetSonar%20marker) false false)
  (Transformation|SetWorldLocation (Variables|Default|GetSonar%20marker) (Transformation|GetWorldLocation (Variables|Components|GetCone_Sonar)) false false))

(event Collision|EventActorBeginOverlap
  (params (OtherActor :type Actor%20Object%20Reference)))

(event EventTick
  (params (DeltaSeconds :type Float%20%28single-precision%29))
  (Rendering|Material|SetVectorParameterValue "/Game/Sonar/MaterialParameterCollection/MPC_Sonar.MPC_Sonar" "EmitterPos" (Math|Conversions|ToLinearColor(Vector) (Transformation|GetWorldLocation (Variables|Components|GetCone_Sonar))) :!class /Script/Engine.KismetMaterialLibrary)
  (Rendering|Material|SetVectorParameterValue "/Game/Sonar/MaterialParameterCollection/MPC_Sonar.MPC_Sonar" "SonarDirWS" (Math|Conversions|ToLinearColor(Vector) (Transformation|GetActorForwardVector)) :!class /Script/Engine.KismetMaterialLibrary)
  (Rendering|Material|SetScalarParameterValue "/Game/Sonar/MaterialParameterCollection/MPC_Sonar.MPC_Sonar" "Range" (Variables|Default|GetRange) :!class /Script/Engine.KismetMaterialLibrary)
  (Rendering|Material|SetScalarParameterValue "/Game/Sonar/MaterialParameterCollection/MPC_Sonar.MPC_Sonar" "HalfAngleDeg" (Variables|Default|GetHalfAngleDeg) :!class /Script/Engine.KismetMaterialLibrary)
  (Rendering|Material|SetScalarParameterValue "/Game/Sonar/MaterialParameterCollection/MPC_Sonar.MPC_Sonar" "PingHz" (Variables|Default|GetPingHz) :!class /Script/Engine.KismetMaterialLibrary)
  (Rendering|Material|SetScalarParameterValue "/Game/Sonar/MaterialParameterCollection/MPC_Sonar.MPC_Sonar" "NoiseAmp" (Variables|Default|GetNoiseAmp) :!class /Script/Engine.KismetMaterialLibrary)
  (Rendering|Material|SetScalarParameterValue "/Game/Sonar/MaterialParameterCollection/MPC_Sonar.MPC_Sonar" "IMU_DriftRate" (Variables|Default|GetIMU_DriftRate) :!class /Script/Engine.KismetMaterialLibrary)
  (Rendering|Material|SetScalarParameterValue "/Game/Sonar/MaterialParameterCollection/MPC_Sonar.MPC_Sonar" "Mode" (Variables|Default|GetMode) :!class /Script/Engine.KismetMaterialLibrary))

(fn ConstructionScript)