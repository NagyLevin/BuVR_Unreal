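; Sonar emitter actor that drives the shared MPC_Sonar parameter collection and a Niagara point cloud.
; BeginPlay sets the cloud's spawn count from the ray count, restarts it after a short delay, and seeds sonar settings from the collection.
; Tick publishes the cone's position, actor forward vector and those settings back to the collection.
; Ping toggling and IMU drift logic are disconnected, and DoPing is an empty stub.
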(event Custom|DoPing
  (if (Variables|Default|GetAutoPing)
    _))

(event EventBeginPlay
  (bind _returnvalue (Rendering|Material|GetScalarParameterValue "/Game/Sonar/MaterialParameterCollection/MPC_Sonar.MPC_Sonar" "Light" :!class /Script/Engine.KismetMaterialLibrary))
  (if (== _returnvalue 0.0)
    (Variables|Default|SetLights false)
    (else
      (Variables|Default|SetLights true)))
  (Class|NiagaraComponent|SetVariableInt (Variables|Default|GetNS_SonarPointCloud) "SpawnCount" (Math|Float|Truncate (Variables|Default|GetNumRays_BP)))
  (Utilities|FlowControl|Delay 0.0)
  (Components|Activation|Activate (Variables|Default|GetNS_SonarPointCloud) false)
  (Utilities|FlowControl|Delay 0.2)
  (Niagara|ReinitializeSystem (Variables|Default|GetNS_SonarPointCloud))
  (bind _returnvalue_2 (Rendering|Material|GetScalarParameterValue "/Game/Sonar/MaterialParameterCollection/MPC_Sonar.MPC_Sonar" "HalfAngleDeg" :!class /Script/Engine.KismetMaterialLibrary))
  (Variables|Default|SetHalfAngleDeg _returnvalue_2)
  (bind _returnvalue_3 (Rendering|Material|GetScalarParameterValue "/Game/Sonar/MaterialParameterCollection/MPC_Sonar.MPC_Sonar" "IMU_DriftRate" :!class /Script/Engine.KismetMaterialLibrary))
  (Variables|Default|SetIMU_DriftRate _returnvalue_3)
  (bind _returnvalue_4 (Rendering|Material|GetScalarParameterValue "/Game/Sonar/MaterialParameterCollection/MPC_Sonar.MPC_Sonar" "Mode" :!class /Script/Engine.KismetMaterialLibrary))
  (Variables|Default|SetMode _returnvalue_4)
  (bind _returnvalue_5 (Rendering|Material|GetScalarParameterValue "/Game/Sonar/MaterialParameterCollection/MPC_Sonar.MPC_Sonar" "NoiseAmp" :!class /Script/Engine.KismetMaterialLibrary))
  (Variables|Default|SetNoiseAmp _returnvalue_5)
  (bind _returnvalue_6 (Rendering|Material|GetScalarParameterValue "/Game/Sonar/MaterialParameterCollection/MPC_Sonar.MPC_Sonar" "PingHz" :!class /Script/Engine.KismetMaterialLibrary))
  (Variables|Default|SetPingHz _returnvalue_6)
  (bind _returnvalue_7 (Rendering|Material|GetScalarParameterValue "/Game/Sonar/MaterialParameterCollection/MPC_Sonar.MPC_Sonar" "Range" :!class /Script/Engine.KismetMaterialLibrary))
  (Variables|Default|SetRange _returnvalue_7))

(event Collision|EventActorBeginOverlap
  (params (OtherActor :type Actor%20Object%20Reference)))

(event EventTick
  (params (DeltaSeconds :type Float%20%28single-precision%29))
  (Rendering|Material|SetVectorParameterValue "/Game/Sonar/MaterialParameterCollection/MPC_Sonar.MPC_Sonar" "EmitterPos" (Math|Conversions|ToLinearColor(Vector) (Transformation|GetWorldLocation (Variables|Components|GetCone))) :!class /Script/Engine.KismetMaterialLibrary)
  (Rendering|Material|SetVectorParameterValue "/Game/Sonar/MaterialParameterCollection/MPC_Sonar.MPC_Sonar" "SonarDirWS" (Math|Conversions|ToLinearColor(Vector) (Transformation|GetActorForwardVector)) :!class /Script/Engine.KismetMaterialLibrary)
  (Rendering|Material|SetScalarParameterValue "/Game/Sonar/MaterialParameterCollection/MPC_Sonar.MPC_Sonar" "Range" (Variables|Default|GetRange) :!class /Script/Engine.KismetMaterialLibrary)
  (Rendering|Material|SetScalarParameterValue "/Game/Sonar/MaterialParameterCollection/MPC_Sonar.MPC_Sonar" "HalfAngleDeg" (Variables|Default|GetHalfAngleDeg) :!class /Script/Engine.KismetMaterialLibrary)
  (Rendering|Material|SetScalarParameterValue "/Game/Sonar/MaterialParameterCollection/MPC_Sonar.MPC_Sonar" "PingHz" (Variables|Default|GetPingHz) :!class /Script/Engine.KismetMaterialLibrary)
  (Rendering|Material|SetScalarParameterValue "/Game/Sonar/MaterialParameterCollection/MPC_Sonar.MPC_Sonar" "NoiseAmp" (Variables|Default|GetNoiseAmp) :!class /Script/Engine.KismetMaterialLibrary)
  (Rendering|Material|SetScalarParameterValue "/Game/Sonar/MaterialParameterCollection/MPC_Sonar.MPC_Sonar" "IMU_DriftRate" (Variables|Default|GetIMU_DriftRate) :!class /Script/Engine.KismetMaterialLibrary)
  (Rendering|Material|SetScalarParameterValue "/Game/Sonar/MaterialParameterCollection/MPC_Sonar.MPC_Sonar" "Mode" (Variables|Default|GetMode) :!class /Script/Engine.KismetMaterialLibrary))

(fn ConstructionScript)