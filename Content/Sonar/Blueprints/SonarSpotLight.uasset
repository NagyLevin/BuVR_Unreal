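; Sonar spotlight Blueprint that switches its light on and off with the ToggleLight input action.
; A FlipFlop alternates off and on, starting with off, setting the spotlight intensity, writing the "Light" scalar in the MPC_Sonar material parameter collection and printing the state.
; Tick reads that shared parameter back every frame and sets the intensity to match, so the collection value drives the light.
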(event EventBeginPlay)

(event Collision|EventActorBeginOverlap
  (params (OtherActor :type Actor%20Object%20Reference)))

(event EventTick
  (params (DeltaSeconds :type Float%20%28single-precision%29))
  (bind _returnvalue (Rendering|Material|GetScalarParameterValue "/Game/Sonar/MaterialParameterCollection/MPC_Sonar.MPC_Sonar" "Light" :!class /Script/Engine.KismetMaterialLibrary))
  (if (== _returnvalue 0.0)
    (Rendering|Components|Light|SetIntensity (Variables|Default|GetSpotLight) 0.0)
    (else
      (Rendering|Components|Light|SetIntensity (Variables|Default|GetSpotLight) 1.6e+02))))

(event Input|ActionEvents|InputActionToggleLight
  (params (Key :type Key%20Structure :default "None"))
  (:Pressed
    (Utilities|FlowControl|FlipFlop
      (:A
        (Rendering|Components|Light|SetIntensity (Variables|Default|GetSpotLight) 0.0)
        (Rendering|Material|SetScalarParameterValue "/Game/Sonar/MaterialParameterCollection/MPC_Sonar.MPC_Sonar" "Light" 0.0 :!class /Script/Engine.KismetMaterialLibrary)
        (Development|PrintString "Light OFF"))
      (:B
        (Rendering|Components|Light|SetIntensity (Variables|Default|GetSpotLight) 1.6e+02)
        (Rendering|Material|SetScalarParameterValue "/Game/Sonar/MaterialParameterCollection/MPC_Sonar.MPC_Sonar" "Light" 1.0 :!class /Script/Engine.KismetMaterialLibrary)
        (Development|PrintString "Light ON")))))

(fn ConstructionScript)