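; Sonar emitter that simulates a scanning sonar, spawning Niagara point sprites at detected surfaces.
; A looping timer sweeps a fan of line traces, refining floor hits with stepped, widening box traces and injecting random noise.
; Beyond a drift threshold, returns plot around a locked, marked origin until re-locked, also holding rotation during fast movement.
; MPC_Sonar supplies tuning and re-lock requests, and receives emitter position and direction each tick.
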(event Custom|Debug
  ;[0.15 0.15 0.15 0.5] Debug Zone
)

(event Custom|DoPing
  (bind _returnvalue (Math|Vector|MakeVector 0.0 0.0 1.0))
  (bind _cone_sonar (Variables|Components|GetCone_Sonar))
  (bind _cone_sonar_2 (Variables|Components|GetCone_Sonar))
  (bind _cone_sonar_3 (Variables|Components|GetCone_Sonar))
  (bind _cone_sonar_4 (Variables|Components|GetCone_Sonar))
  (bind _returnvalue_2 (Transformation|GetWorldLocation _cone_sonar))
  (bind _returnvalue_3 (Transformation|GetWorldLocation _cone_sonar_3))
  (bind _returnvalue_4 (Transformation|GetWorldRotation _cone_sonar_4))
  ;[0.08929 0.06248 0.15 0.5] Freeze pos Logic
  (Variables|Default|SetE_CurrentEmitterLocation (Transformation|GetWorldLocation (Variables|Components|GetCone_Sonar)))
  (if (Variables|Default|GetE_bLockedLocationInitialized)
    (if (Variables|Default|GetE_FreezeOnLargeTranslation)
      (bind _returnvalue_5 (Rendering|Material|GetScalarParameterValue "/Game/Sonar/MaterialParameterCollection/MPC_Sonar.MPC_Sonar" "S_LockNewPos" :!class /Script/Engine.KismetMaterialLibrary))
      (if (== _returnvalue_5 1.0)
        (Variables|Default|SetE_LockedEmitterLocation (Variables|Default|GetE_CurrentEmitterLocation))
        (Transformation|SetWorldLocation (Variables|Default|GetSonar%20marker) (Variables|Default|GetE_CurrentEmitterLocation) false false)
        (Rendering|Material|SetScalarParameterValue "/Game/Sonar/MaterialParameterCollection/MPC_Sonar.MPC_Sonar" "S_LockNewPos" 0.0 :!class /Script/Engine.KismetMaterialLibrary))
      (else
        (Variables|Default|SetE_TranslationDistance (Math|Vector|Distance(Vector) (Variables|Default|GetE_LockedEmitterLocation) (Variables|Default|GetE_CurrentEmitterLocation)))
        (if (<= (Variables|Default|GetE_TranslationDistance) (Variables|Default|GetE_TranslationThreshold))
          _
          (else
            (Rendering|SetVisibility (Variables|Default|GetSonar%20marker) true false)
            (Variables|Default|SetE_FreezeOnLargeTranslation true)))))
    (else
      (Variables|Default|SetE_LockedEmitterLocation (Variables|Default|GetE_CurrentEmitterLocation))
      (Variables|Default|SetE_bLockedLocationInitialized true)))
  ;[0.15 0.15 0.15 0.5] Velocity
  (if (> (/ (Math|Vector|Distance(Vector) _returnvalue_3 (Variables|Default|GetH_PervLoc)) 0.05) (Variables|Default|GetH_MAxSpeed))
    (Variables|Default|SetH_FreezeLoc true)
    (else
      (Variables|Default|SetH_FreezeLoc false)))
  (Variables|Default|SetH_PervLoc _returnvalue_3)
  ;[0.15 0.6957 0.15 0.5] Sonar Spread
  (bind _returnvalue_6 (Rendering|Material|GetScalarParameterValue "/Game/Sonar/MaterialParameterCollection/MPC_Sonar.MPC_Sonar" "S_Fov" :!class /Script/Engine.KismetMaterialLibrary))
  (Variables|Default|SetS_FOVAngle (/ _returnvalue_6 2.0))
  (for _index (range 0 (- (Variables|Default|GetS_Numrays) -1))
    (Variables|Default|SetS_RayHitLoc _returnvalue_2)
    (Variables|Default|SetE_DisplayPoint _returnvalue_2)
    (Variables|Default|SetE_DirectionVector (Math|Vector|RotateVectorAroundAxis (Math|Vector|GetForwardVector _cone_sonar_2) (Math|Float|MapRangeClamped (Math|Conversions|ToFloat(Integer) _index) 0.0 (Math|Conversions|ToFloat(Integer) (- (Variables|Default|GetS_Numrays) -1)) (* (* (Variables|Default|GetS_FOVAngle) 0.3) -1.0) (* (Variables|Default|GetS_FOVAngle) 0.3)) (Math|Vector|GetRightVector _cone_sonar_2)))
    ;[0.03833 0.1321 0.15 0.5] LineTrace
    (bind (_outhit _returnvalue_7) (Collision|LineTraceByChannel (Variables|Default|GetE_CurrentEmitterLocation) (+ (* (Variables|Default|GetE_DirectionVector) (Variables|Default|GetS_MaxRange)) (Variables|Default|GetE_CurrentEmitterLocation)) "TraceTypeQuery1" false 0 "None"))
    (if _returnvalue_7
      (if (Actor|ActorHasTag (.HitActor (Collision|BreakHitResult _outhit)) "Floor")
        (Variables|Default|SetS_RayHitLoc (.Location (Collision|BreakHitResult _outhit)))
        (Variables|Default|SetE_DisplayPoint (.Location (Collision|BreakHitResult _outhit)))
        ;[0.15 0.05966 0.1051 0.5] BOXTRACE
        (bind _index_2 (Utilities|FlowControl|ForLoopwithBreak 1 (Variables|Default|GetS_steps) :!label _label)
          (:LoopBody
            (if (> (Math|Float|Absolute(Float) (Math|Vector|DotProduct (Math|Vector|GetRightVector _returnvalue_4) _returnvalue)) (Math|Float|Absolute(Float) (Math|Vector|DotProduct (Math|Vector|GetUpVector _returnvalue_4) _returnvalue)))
              (Variables|Default|SetE_WidehitboxZ (* (* (Math|Conversions|ToFloat(Integer) _index_2) 2e+02) 0.1))
              (else
                (Variables|Default|SetE_WidehitboxY (* (* (Math|Conversions|ToFloat(Integer) _index_2) 2e+02) 0.1))))
            (bind (_outhit_2 _returnvalue_8) (Collision|BoxTraceByChannel (+ (Variables|Default|GetE_CurrentEmitterLocation) (* (Variables|Default|GetE_DirectionVector) (* (Math|Conversions|ToFloat(Integer) (- _index_2 1)) 2e+02))) (+ (* (* (Math|Conversions|ToFloat(Integer) _index_2) 2e+02) (Variables|Default|GetE_DirectionVector)) (Variables|Default|GetE_CurrentEmitterLocation)) (Math|Vector|MakeVector 1.0 (* (Variables|Default|GetE_WidehitboxY) (Variables|Default|GetB_NoiseHitboxSize)) 0.0) (Math|Rotator|MakeRotfromZX (Math|Vector|GetUpVector (Transformation|GetWorldRotation (Variables|Components|GetCone_Sonar))) (Variables|Default|GetE_DirectionVector)) "TraceTypeQuery1" false 0 "None"))
            ;[0.15 0.15 0.15 0.5] Random noise boxtrace
            (bind _returnvalue_9 (Rendering|Material|GetScalarParameterValue "/Game/Sonar/MaterialParameterCollection/MPC_Sonar.MPC_Sonar" "S_NoiseRange" :!class /Script/Engine.KismetMaterialLibrary))
            (if (< (Math|Random|RandomFloatinRange 0.001 1.0) (/ _returnvalue_9 1e+01))
              (Variables|Default|SetE_DisplayPoint (+ (Variables|Default|GetE_LockedEmitterLocation) (* (Variables|Default|GetE_DirectionVector) (* (Math|Random|RandomFloatinRange 0.0 1.0) (Variables|Default|GetS_MaxRange)))))
              ;[0.15 0.01394 0.01573 0.5] Display the Sprites
              (Rendering|Debug|DrawDebugLine "0, 0, 0" "0, 0, 0" "(R=0.000000,G=1.000000,B=0.000000,A=1.000000)" 1.0 1.0 :!label _label_2)
              (Rendering|Debug|DrawDebugLine "0, 0, 0" "0, 0, 0" "(R=1.000000,G=0.000000,B=0.000000,A=1.000000)" 1.0 1.0)
              (if (> (Math|Vector|Distance(Vector) (Variables|Default|GetE_CurrentEmitterLocation) (Variables|Default|GetE_DisplayPoint)) 1.0)
                (Niagara|SpawnSystematLocation "/Game/Sonar/NS_Sonar_Raycast.NS_Sonar_Raycast" (Variables|Default|GetE_DisplayPoint)))
              (elif _returnvalue_8
                (if (Actor|ActorHasTag (.HitActor (Collision|BreakHitResult _outhit_2)) "Floor")
                  (goto _label Break)
                  (else
                    (Variables|Default|SetS_RayHitLoc (.Location (Collision|BreakHitResult _outhit_2)))
                    (Variables|Default|SetE_DisplayPoint (+ (+ (.ImpactPoint (Collision|BreakHitResult _outhit_2)) (* (Math|Vector|GetRightVector (Math|Rotator|MakeRotfromX (Variables|Default|GetE_DirectionVector))) (* (* (* (Variables|Default|GetE_WidehitboxZ) (Variables|Default|GetE_WidehitboxY)) 1.0) (Math|Float|Sign(Float) (Math|Vector|DotProduct (- (.Location (Collision|BreakHitResult _outhit_2)) (.ImpactPoint (Collision|BreakHitResult _outhit_2))) (Math|Vector|GetRightVector (Math|Rotator|MakeRotfromX (Variables|Default|GetE_DirectionVector)))))))) (* (Variables|Default|GetE_DirectionVector) (Variables|Default|GetL_OffsetDistance))))
                    (goto _label Break))))))
          (:Completed
            ;[0.001747 0.1198 0.15 0.5] Freeze rotation when large translation
            (if (Variables|Default|GetE_FreezeOnLargeTranslation)
              ;[0.15 0.15 0.15 0.5] Pivot between rotation onli and no rotation
              (if (Variables|Default|GetH_FreezeLoc) :!label _label_3
                ;[0.15 0.15 0.15 0.5] Hit event without rot
                (Variables|Default|SetE_DisplayPoint (+ (Math|Vector|RotateVector (Math|Vector|UnrotateVector (- (Variables|Default|GetS_RayHitLoc) (Variables|Default|GetE_CurrentEmitterLocation)) (Transformation|GetWorldRotation (Variables|Components|GetCone_Sonar))) (Math|Rotator|MakeRotator (.roll (Variables|Default|GetB_RotbeforeFreeze)) (.pitch (Variables|Default|GetB_RotbeforeFreeze)) (.yaw (Variables|Default|GetB_RotbeforeFreeze)))) (Variables|Default|GetE_LockedEmitterLocation)))
                (goto _label_2)
                (else
                  (Variables|Default|SetB_RotbeforeFreeze (Transformation|GetWorldRotation (Variables|Components|GetCone_Sonar)))
                  ;[0.15 0.15 0.15 0.5] Hit event with rot
                  (Variables|Default|SetE_DisplayPoint (+ (- (Variables|Default|GetS_RayHitLoc) (Variables|Default|GetE_CurrentEmitterLocation)) (Variables|Default|GetE_LockedEmitterLocation)))
                  (goto _label_2)))
              (else
                (goto _label_2)))))
        (else
          (Variables|Default|SetS_RayHitLoc (.Location (Collision|BreakHitResult _outhit)))
          (Variables|Default|SetE_DisplayPoint (.Location (Collision|BreakHitResult _outhit)))
          (if (Variables|Default|GetE_FreezeOnLargeTranslation)
            (goto _label_3)
            (else
              ;[0.15 0.15 0.15 0.5] Random noise linetrace
              (bind _returnvalue_10 (Rendering|Material|GetScalarParameterValue "/Game/Sonar/MaterialParameterCollection/MPC_Sonar.MPC_Sonar" "S_NoiseRange" :!class /Script/Engine.KismetMaterialLibrary))
              (if (< (Math|Random|RandomFloatinRange 0.001 1.0) (/ _returnvalue_10 1e+01))
                (Variables|Default|SetE_DisplayPoint (+ (Variables|Default|GetE_LockedEmitterLocation) (* (Variables|Default|GetE_DirectionVector) (* (Math|Random|RandomFloatinRange 0.0 1.0) (Variables|Default|GetS_MaxRange)))))
                (goto _label_2)
                (else
                  (goto _label_2)))))))
      (else
        (goto _label)))))

(event EventBeginPlay
  (bind _cone_sonar (Variables|Components|GetCone_Sonar))
  (bind _returnvalue (Transformation|GetWorldLocation _cone_sonar))
  ;[0.15 0.15 0.15 0.5] Sync this first(warmup)
  (bind _returnvalue_2 (Rendering|Material|GetScalarParameterValue "/Game/Sonar/MaterialParameterCollection/MPC_Sonar.MPC_Sonar" "Light" :!class /Script/Engine.KismetMaterialLibrary))
  (if (== _returnvalue_2 0.0)
    (Variables|Default|SetLights false)
    (else
      (Variables|Default|SetLights true)))
  (bind _returnvalue_3 (Rendering|Material|GetScalarParameterValue "/Game/Sonar/MaterialParameterCollection/MPC_Sonar.MPC_Sonar" "HalfAngleDeg" :!class /Script/Engine.KismetMaterialLibrary))
  (Variables|Default|SetHalfAngleDeg _returnvalue_3)
  (bind _returnvalue_4 (Rendering|Material|GetScalarParameterValue "/Game/Sonar/MaterialParameterCollection/MPC_Sonar.MPC_Sonar" "IMU_DriftRate" :!class /Script/Engine.KismetMaterialLibrary))
  (Variables|Default|SetIMU_DriftRate _returnvalue_4)
  (bind _returnvalue_5 (Rendering|Material|GetScalarParameterValue "/Game/Sonar/MaterialParameterCollection/MPC_Sonar.MPC_Sonar" "Mode" :!class /Script/Engine.KismetMaterialLibrary))
  (Variables|Default|SetMode _returnvalue_5)
  (bind _returnvalue_6 (Rendering|Material|GetScalarParameterValue "/Game/Sonar/MaterialParameterCollection/MPC_Sonar.MPC_Sonar" "NoiseAmp" :!class /Script/Engine.KismetMaterialLibrary))
  (Variables|Default|SetNoiseAmp _returnvalue_6)
  (bind _returnvalue_7 (Rendering|Material|GetScalarParameterValue "/Game/Sonar/MaterialParameterCollection/MPC_Sonar.MPC_Sonar" "PingHz" :!class /Script/Engine.KismetMaterialLibrary))
  (Variables|Default|SetPingHz _returnvalue_7)
  (bind _returnvalue_8 (Rendering|Material|GetScalarParameterValue "/Game/Sonar/MaterialParameterCollection/MPC_Sonar.MPC_Sonar" "Range" :!class /Script/Engine.KismetMaterialLibrary))
  (Variables|Default|SetRange _returnvalue_8)
  (Utilities|Time|SetTimerbyFunctionName 0 "DoPing" 0.05 true)
  (Utilities|Time|SetTimerbyFunctionName 0 "Debug" 0.5 true)
  (Transformation|SetWorldRotation (Variables|Components|GetCone_Sonar) (Transformation|GetActorRotation) false false)
  (Variables|Default|SetE_LockedEmitterLocation (Transformation|GetWorldLocation (Variables|Components|GetCone_Sonar)))
  (Variables|Default|SetE_bLockedLocationInitialized true)
  ;;[0.15 0.15 0.15 0.5] Make reference cone invis
  (Rendering|SetVisibility (Variables|Default|GetSonar%20marker) false false)
  (Transformation|SetWorldLocation (Variables|Default|GetSonar%20marker) _returnvalue false false)
  (Variables|Default|SetH_PervLoc _returnvalue))

(event EventTick
  (params (DeltaSeconds :type Float%20%28single-precision%29))
  ;[0.15 0.15 0.15 0.5] Offten synced values
  (Rendering|Material|SetVectorParameterValue "/Game/Sonar/MaterialParameterCollection/MPC_Sonar.MPC_Sonar" "EmitterPos" (Math|Conversions|ToLinearColor(Vector) (Transformation|GetWorldLocation (Variables|Components|GetCone_Sonar))) :!class /Script/Engine.KismetMaterialLibrary)
  (Rendering|Material|SetVectorParameterValue "/Game/Sonar/MaterialParameterCollection/MPC_Sonar.MPC_Sonar" "SonarDirWS" (Math|Conversions|ToLinearColor(Vector) (Transformation|GetActorForwardVector)) :!class /Script/Engine.KismetMaterialLibrary)
  (bind _returnvalue (Rendering|Material|GetScalarParameterValue "/Game/Sonar/MaterialParameterCollection/MPC_Sonar.MPC_Sonar" "S_NoiseHitbox" :!class /Script/Engine.KismetMaterialLibrary))
  (Variables|Default|SetB_NoiseHitboxSize _returnvalue))

(fn ConstructionScript)