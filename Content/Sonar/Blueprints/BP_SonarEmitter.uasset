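; Sonar emitter actor that pings a Niagara point cloud on a looping timer, with the Ping input toggling it.
; Each tick it writes its position and forward vector to MPC_Sonar and reads sonar settings back from that collection.
; Mode 2 offsets the position by accumulated IMU drift and noise, and overwrites direction with actor location; other modes ease drift toward zero.
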(event Custom|DoPing
  (if (Variables|Default|GetAutoPing)
    (Class|NiagaraComponent|SetVariableInt (Variables|Default|GetNS_SonarPointCloud) "SpawnCount" (Math|Float|Truncate (Variables|Default|GetNumRays_BP)))
    (Utilities|FlowControl|Delay 0.0)
    (Components|Activation|Activate (Variables|Default|GetNS_SonarPointCloud) false)
    (Utilities|FlowControl|Delay 0.2)
    (Niagara|ReinitializeSystem (Variables|Default|GetNS_SonarPointCloud))))

(event EventBeginPlay
  (if (Variables|Default|GetAutoPing)
    (bind _returnvalue (Utilities|Time|SetTimerbyFunctionName 0 "DoPing" (Variables|Default|GetPingInterval) true))
    (Variables|Default|SetPingTimerHandle _returnvalue)))

(event Collision|EventActorBeginOverlap
  (params (OtherActor :type Actor%20Object%20Reference)))

(event EventTick
  (params (DeltaSeconds :type Float%20%28single-precision%29))
  (bind _returnvalue (Transformation|GetActorLocation))
  (Rendering|Material|SetVectorParameterValue "/Game/Sonar/MaterialParameterCollection/MPC_Sonar.MPC_Sonar" "EmitterPos" (Math|Conversions|ToLinearColor(Vector) (Transformation|GetActorLocation)) :!class /Script/Engine.KismetMaterialLibrary)
  (Rendering|Material|SetVectorParameterValue "/Game/Sonar/MaterialParameterCollection/MPC_Sonar.MPC_Sonar" "SonarDirWS" (Math|Conversions|ToLinearColor(Vector) (Transformation|GetActorForwardVector)) :!class /Script/Engine.KismetMaterialLibrary)
  (bind _returnvalue_2 (Rendering|Material|GetScalarParameterValue "/Game/Sonar/MaterialParameterCollection/MPC_Sonar.MPC_Sonar" "HalfAngleDeg" :!class /Script/Engine.KismetMaterialLibrary))
  (Variables|Default|SetHalfAngleDeg _returnvalue_2)
  (bind _returnvalue_3 (Rendering|Material|GetScalarParameterValue "/Game/Sonar/MaterialParameterCollection/MPC_Sonar.MPC_Sonar" "IMU_DriftRate" :!class /Script/Engine.KismetMaterialLibrary))
  (Variables|Default|SetIMU_DriftRate _returnvalue_3)
  (bind _returnvalue_4 (Rendering|Material|GetScalarParameterValue "/Game/Sonar/MaterialParameterCollection/MPC_Sonar.MPC_Sonar" "Mode" :!class /Script/Engine.KismetMaterialLibrary))
  (Variables|Default|SetMode _returnvalue_4)
  (bind _returnvalue_5 (Rendering|Material|GetScalarParameterValue "/Game/Sonar/MaterialParameterCollection/MPC_Sonar.MPC_Sonar" "NoiseAmp" :!class /Script/Engine.KismetMaterialLibrary))
  (Variables|Default|SetNoiseAmp _returnvalue_5)
  (bind _returnvalue_6 (Rendering|Material|GetScalarParameterValue "/Game/Sonar/MaterialParameterCollection/MPC_Sonar.MPC_Sonar" "PingHz" :!class /Script/Engine.KismetMaterialLibrary))
  (Variables|Default|SetPingHz _returnvalue_6)
  (bind _returnvalue_7 (Rendering|Material|GetScalarParameterValue "/Game/Sonar/MaterialParameterCollection/MPC_Sonar.MPC_Sonar" "Range" :!class /Script/Engine.KismetMaterialLibrary))
  (Variables|Default|SetRange _returnvalue_7)
  (if (== (Variables|Default|GetMode) 2.0)
    (Variables|Default|SetDriftVec (+ (* (Transformation|GetActorForwardVector) (Variables|Default|GetIMU_DriftRate) (Utilities|Time|GetWorldDeltaSeconds)) (* (Math|Random|RandomUnitVector) (Variables|Default|GetNoiseAmp) (Variables|Default|Get0,1) (Utilities|Time|GetWorldDeltaSeconds)) (Variables|Default|GetDriftVec)))
    (Rendering|Material|SetVectorParameterValue "/Game/Sonar/MaterialParameterCollection/MPC_Sonar.MPC_Sonar" "EmitterPos" (Math|Conversions|ToLinearColor(Vector) (Math|Vector|SelectVector (+ (Variables|Default|GetDriftVec) _returnvalue) _returnvalue (== (Variables|Default|GetMode) 2.0))) :!class /Script/Engine.KismetMaterialLibrary)
    (Rendering|Material|SetVectorParameterValue "/Game/Sonar/MaterialParameterCollection/MPC_Sonar.MPC_Sonar" "SonarDirWS" (Math|Conversions|ToLinearColor(Vector) _returnvalue) :!class /Script/Engine.KismetMaterialLibrary)
    (else
      (Variables|Default|SetDriftVec (Math|Interpolation|VInterpTo (Variables|Default|GetDriftVec) (Math|Vector|MakeVector 0.0 0.0 0.0) (Utilities|Time|GetWorldDeltaSeconds) 0.5)))))

(event Input|ActionEvents|InputActionPing
  (params (Key :type Key%20Structure :default "None"))
  (:Pressed
    (if (Variables|Default|GetbSonarOn)
      (Utilities|Time|ClearandInvalidateTimerbyHandle (Variables|Default|GetPingTimerHandle))
      (Variables|Default|SetbSonarOn false)
      (Variables|Default|SetAutoPing false)
      (else
        (Utilities|Time|SetTimerbyFunctionName 0 "DoPing" (Variables|Default|GetPingInterval) true)
        (Variables|Default|SetbSonarOn true)
        (Variables|Default|SetAutoPing true)))))

(fn ConstructionScript)